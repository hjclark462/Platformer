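; BP_Message is a trigger volume that shows a text message, passed as tutorial text, on the HUD.
; Box overlap begin and end set InBox to Visible or Hidden, with hiding delayed four seconds.
; Both events find top-level BP_Widget_HUD widgets and pass InBox and the text to their OnMessage.
; The player tag checks are unconnected, so overlaps are not filtered by tag.
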(event `self.Box.OnComponentBeginOverlap`
  (params (OverlappedComponent :type "PrimitiveComponent Object Reference") (OtherActor :type "Actor Object Reference") (OtherComp :type "PrimitiveComponent Object Reference") (OtherBodyIndex :type Integer) (bFromSweep :type Boolean) (SweepResult :type "HitResult Structure (by ref)"))
  (set `self.InBox` "Visible")
  (bind _foundwidgets (`WidgetBlueprintLibrary.GetAllWidgetsOfClass` "/Game/_MyContent/UI/BP_Widget_HUD.BP_Widget_HUD_C"))
  (`/Game/_MyContent/UI/BP_Widget_HUD.OnMessage` _foundwidgets (`self.InBox`) (`self.Messsage Text`)))

(event `self.Box.OnComponentEndOverlap`
  (params (OverlappedComponent :type "PrimitiveComponent Object Reference") (OtherActor :type "Actor Object Reference") (OtherComp :type "PrimitiveComponent Object Reference") (OtherBodyIndex :type Integer))
  (`KismetSystemLibrary.Delay` 4.0)
  (set `self.InBox` "Hidden")
  (bind _foundwidgets (`WidgetBlueprintLibrary.GetAllWidgetsOfClass` "/Game/_MyContent/UI/BP_Widget_HUD.BP_Widget_HUD_C"))
  (`/Game/_MyContent/UI/BP_Widget_HUD.OnMessage` _foundwidgets (`self.InBox`) (`self.Messsage Text`)))

(fn `UserConstructionScript`)