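; BP_HPUP is a spinning health pickup that adds HealthPoint to a ThirdPersonCharacter overlapping its box.
; On pickup it updates the game manager's health widget with HealthPoints divided by 100, without clamping.
; It then hides itself and disables collision, respawning after a ten-second delay rather than being destroyed.
; Construction stores a display-name UID and caches BP_MyGameManager if exactly one exists; DestroyCollectable separately destroys the actor.
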(event `self.ReceiveTick`
  (params (DeltaSeconds :type "Float (single-precision)"))
  (`self.K2_AddActorLocalRotation` (struct :`Yaw` 1.0)))

(event `self.Box.OnComponentBeginOverlap`
  (params (OverlappedComponent :type "PrimitiveComponent Object Reference") (OtherActor :type "Actor Object Reference") (OtherComp :type "PrimitiveComponent Object Reference") (OtherBodyIndex :type Integer) (bFromSweep :type Boolean) (SweepResult :type "HitResult Structure (by ref)"))
  (bind _asthird_person_character (cast `/Game/ThirdPersonBP/Blueprints/ThirdPersonCharacter` OtherActor))
  (bind _output_get (set `/Game/ThirdPersonBP/Blueprints/ThirdPersonCharacter.Health Points` (+ (`/Game/ThirdPersonBP/Blueprints/ThirdPersonCharacter.Health Points` _asthird_person_character) (`self.HealthPoint+`)) _asthird_person_character))
  (bind _my_game_manager (`/Game/_MyContent/Blueprints/BP_MyFunctionLibrary.Get My Game Manager`))
  (set `/Game/_MyContent/UI/BP_Widget_Health.Health` (/ _output_get 100.0) (`/Game/_MyContent/Blueprints/BP_MyGameManager.Widget_Health` _my_game_manager))
  (`PrimitiveComponent.SetCollisionEnabled` (`self.Box`) "NoCollision")
  (`SceneComponent.SetVisibility` (`self.DefaultSceneRoot`) false true)
  (`KismetSystemLibrary.Delay` 10.0)
  (`PrimitiveComponent.SetCollisionEnabled` (`self.Box`) "QueryAndPhysics")
  (`SceneComponent.SetVisibility` (`self.DefaultSceneRoot`) true true))

(fn `CreateUID`
  (set `self.UID` (`KismetSystemLibrary.GetDisplayName` self)))

(fn `DestroyCollectable`
  (`self.K2_DestroyActor`))

(fn `UserConstructionScript`
  (`self.CreateUID`)
  (bind _outactors (`GameplayStatics.GetAllActorsOfClass` "/Game/_MyContent/Blueprints/BP_MyGameManager.BP_MyGameManager_C"))
  (if (== (`KismetArrayLibrary.Array_Length` _outactors) 1)
    (set `self.GameManager` (`|GetArrayItem` _outactors))))