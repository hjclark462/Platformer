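; BP_Jetdash is a pickup that unlocks the jetdash ability for the player character.
; It spins slightly every tick, and when a ThirdPersonCharacter overlaps its box it sets that character's GotJetdash flag and destroys itself.
; The construction script stores the display name as a UID and caches the BP_MyGameManager if exactly one exists, though neither is used elsewhere in this Blueprint.
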(event `self.ReceiveTick`
  (params (DeltaSeconds :type "Float (single-precision)"))
  (`self.K2_AddActorLocalRotation` (struct :`Yaw` 1.0)))

(event `self.Box.OnComponentBeginOverlap`
  (params (OverlappedComponent :type "PrimitiveComponent Object Reference") (OtherActor :type "Actor Object Reference") (OtherComp :type "PrimitiveComponent Object Reference") (OtherBodyIndex :type Integer) (bFromSweep :type Boolean) (SweepResult :type "HitResult Structure (by ref)"))
  (bind _asthird_person_character (cast `/Game/ThirdPersonBP/Blueprints/ThirdPersonCharacter` OtherActor))
  (set `/Game/ThirdPersonBP/Blueprints/ThirdPersonCharacter.GotJetdash` true _asthird_person_character)
  (`self.K2_DestroyActor`))

(fn `CreateUID`
  (set `self.UID` (`KismetSystemLibrary.GetDisplayName` self)))

(fn `UserConstructionScript`
  (`self.CreateUID`)
  (bind _outactors (`GameplayStatics.GetAllActorsOfClass` "/Game/_MyContent/Blueprints/BP_MyGameManager.BP_MyGameManager_C"))
  (if (== (`KismetArrayLibrary.Array_Length` _outactors) 1)
    (set `self.GameManager` (`|GetArrayItem` _outactors))))