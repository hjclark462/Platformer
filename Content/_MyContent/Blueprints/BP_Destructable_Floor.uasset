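; BP_Destructable_Floor is a floor that breaks apart shortly after an actor overlaps its Box trigger, then replaces itself.
; After a DestroyTime delay, radius damage at the Destructible component's location fractures it, and timed delays then hide and destroy the actor.
; A fresh instance spawns at the same transform immediately after the destroy call.
; Any overlapping actor triggers it, as the player tag check is unconnected.
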(event `self.Box.OnComponentBeginOverlap`
  (params (OverlappedComponent :type "PrimitiveComponent Object Reference") (OtherActor :type "Actor Object Reference") (OtherComp :type "PrimitiveComponent Object Reference") (OtherBodyIndex :type Integer) (bFromSweep :type Boolean) (SweepResult :type "HitResult Structure (by ref)"))
  (bind _destructible (`self.Destructible`))
  (`KismetSystemLibrary.Delay` (`self.DestroyTime`))
  (`DestructibleComponent.ApplyRadiusDamage` _destructible 20.0 (`SceneComponent.K2_GetComponentLocation` _destructible) 20.0 0.0 false)
  (`KismetSystemLibrary.Delay` 3.0)
  (`self.SetActorHiddenInGame` true)
  (`KismetSystemLibrary.Delay` 1.0)
  (`self.K2_DestroyActor`)
  (`|SpawnActorFromClass` "BP_Destructable_Floor_C" (`self.GetTransform`) "Undefined" "OverrideRootScale" null null))

(fn `UserConstructionScript`)