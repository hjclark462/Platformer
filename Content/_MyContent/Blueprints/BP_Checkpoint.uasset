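; Checkpoint trigger that saves the player's transform when its box is overlapped, without filtering the overlapping actor.
; With its Load flag on, it updates or creates a BP_SaveGame in the named slot, marking it loadable.
; It then shows a message on the HUD widget for a few seconds and destroys itself.
; With Load off, it instead clears the saved Load flag, acting as a checkpoint reset.
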(event `self.Box.OnComponentBeginOverlap`
  (params (OverlappedComponent :type "PrimitiveComponent Object Reference") (OtherActor :type "Actor Object Reference") (OtherComp :type "PrimitiveComponent Object Reference") (OtherBodyIndex :type Integer) (bFromSweep :type Boolean) (SweepResult :type "HitResult Structure (by ref)"))
  (bind _player_location (`self.Player Location`))
  (bind _slot_name (`self.Slot Name`))
  (if (`self.Load`)
    (`|ExecutionSequence`
      (:`then_0`
        (bind _asthird_person_character (cast `/Game/ThirdPersonBP/Blueprints/ThirdPersonCharacter` (`GameplayStatics.GetPlayerCharacter` 0)))
        (set `self.Player Location` (`self.GetTransform` _asthird_person_character))
        (`KismetSystemLibrary.PrintString` "Checkpoint Reached"))
      (:`then_1`
        (bind _returnvalue (`GameplayStatics.DoesSaveGameExist` (`self.Slot Name`)))
        (if _returnvalue
          (bind _returnvalue_2 (`GameplayStatics.LoadGameFromSlot` (`self.Slot Name`)))
          (bind _asbp_save_game (cast `/Game/_MyContent/Blueprints/BP_SaveGame` _returnvalue_2))
          (set `/Game/_MyContent/Blueprints/BP_SaveGame.PlayerTransform` _player_location _asbp_save_game)
          (set `/Game/_MyContent/Blueprints/BP_SaveGame.Load` true _asbp_save_game)
          (`GameplayStatics.SaveGameToSlot` _asbp_save_game _slot_name)
          (else
            (bind _returnvalue_3 (`GameplayStatics.CreateSaveGameObject` "/Game/_MyContent/Blueprints/BP_SaveGame.BP_SaveGame_C"))
            (set `/Game/_MyContent/Blueprints/BP_SaveGame.PlayerTransform` _player_location _returnvalue_3)
            (set `/Game/_MyContent/Blueprints/BP_SaveGame.Load` true _returnvalue_3)
            (`GameplayStatics.SaveGameToSlot` _returnvalue_3 _slot_name)))
        (set `self.InBox` "Visible")
        (bind _foundwidgets (`WidgetBlueprintLibrary.GetAllWidgetsOfClass` "/Game/_MyContent/UI/BP_Widget_HUD.BP_Widget_HUD_C"))
        (`/Game/_MyContent/UI/BP_Widget_HUD.OnMessage` _foundwidgets (`self.InBox`) (`self.Messsage Text`))
        (`KismetSystemLibrary.Delay` 4.0)
        (set `self.InBox` "Hidden")
        (bind _foundwidgets_2 (`WidgetBlueprintLibrary.GetAllWidgetsOfClass` "/Game/_MyContent/UI/BP_Widget_HUD.BP_Widget_HUD_C"))
        (`/Game/_MyContent/UI/BP_Widget_HUD.OnMessage` _foundwidgets_2 (`self.InBox`) (`self.Messsage Text`))
        (`self.K2_DestroyActor`)))
    (else
      (bind _returnvalue_4 (`GameplayStatics.LoadGameFromSlot` (`self.Slot Name`)))
      (bind _asbp_save_game_2 (cast `/Game/_MyContent/Blueprints/BP_SaveGame` _returnvalue_4))
      (set `/Game/_MyContent/Blueprints/BP_SaveGame.Load` false _asbp_save_game_2)
      (`GameplayStatics.SaveGameToSlot` _asbp_save_game_2 (`self.Slot Name`))
      (`KismetSystemLibrary.PrintString` "Checkpoint Cleared"))))

(fn `UserConstructionScript`)