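; Spline-following moving platform that starts on BeginPlay and that the player can pause or resume with the Use input while overlapping its Box.
; A timeline at a configurable play rate maps its SplineDistance track to spline length, setting the mesh's world location without sweep and optionally restarting when finished.
; The construction script applies the configurable static mesh and material.
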(event `self.ReceiveBeginPlay`
  (`self.Platform Start`)
  (`self.EnableInput` (`GameplayStatics.GetPlayerController` 0)))

(event `Platform Start`
  (bind _spline (`self.Spline`))
  (`TimelineComponent.SetPlayRate` (`self.Motion Timeline`) (`self.Rate`))
  (bind (_direction _spline_distance) (`Timeline|Motion Timeline` :!via `PlayFromStart` :!label _label)
    (:`Update`
      (`SceneComponent.K2_SetWorldLocation` (`self.Platform Mesh`) (`SplineComponent.GetLocationAtDistanceAlongSpline` _spline (* _spline_distance (`SplineComponent.GetSplineLength` _spline)) "World") false false)
      (set `self.IsPlaying` (`TimelineComponent.IsPlaying` (`self.Motion Timeline`))))
    (:`Finished`
      (if (`self.Loop`)
        (goto _label :!via `PlayFromStart`)))))

(event `self.Box.OnComponentBeginOverlap`
  (params (OverlappedComponent :type "PrimitiveComponent Object Reference") (OtherActor :type "Actor Object Reference") (OtherComp :type "PrimitiveComponent Object Reference") (OtherBodyIndex :type Integer) (bFromSweep :type Boolean) (SweepResult :type "HitResult Structure (by ref)"))
  (set `self.MyPlayer` OtherActor)
  (set `self.IsOverlapped` true))

(event `InputAction|Use` :consume false
  (params (Key :type "Key Structure"))
  (:`Pressed`
    (if (`self.IsOverlapped`)
      (if (`self.IsPlaying`)
        (`self.Stop`)
        (else
          (`self.Start`))))))

(event `self.Box.OnComponentEndOverlap`
  (params (OverlappedComponent :type "PrimitiveComponent Object Reference") (OtherActor :type "Actor Object Reference") (OtherComp :type "PrimitiveComponent Object Reference") (OtherBodyIndex :type Integer))
  (set `self.MyPlayer` OtherActor)
  (set `self.IsOverlapped` false))

(fn `Start`
  (`TimelineComponent.Play` (`self.Motion Timeline`)))

(fn `Stop`
  (bind _motion_timeline (`self.Motion Timeline`))
  (`TimelineComponent.Stop` _motion_timeline)
  (`TimelineComponent.SetPlaybackPosition` _motion_timeline (`TimelineComponent.GetPlaybackPosition` _motion_timeline) false true))

(fn `UserConstructionScript`
  (bind _platform_mesh (`self.Platform Mesh`))
  (`StaticMeshComponent.SetStaticMesh` _platform_mesh (`self.Static Mesh`))
  (`PrimitiveComponent.SetMaterial` _platform_mesh 0 (`self.Material`)))